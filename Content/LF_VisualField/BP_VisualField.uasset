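; BP_VisualField is an actor that visualizes a field of view from a scene capture, using a decal and a debug sphere.
; The construction script sizes both to the max distance and creates an R16f render target for the capture, presumably holding depth.
; SetCameraParameters feeds that texture, FOV, range, aspect ratio and camera world position and axes to both dynamic materials.
; Camera values are set only at construction, with no runtime update.
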(fn `SetCameraParameters`
  (params (Mat :type "MaterialInstanceDynamic Object Reference"))
  (bind _scenecapturecomponent2d (`self.SceneCaptureComponent2D`))
  (`MaterialInstanceDynamic.SetTextureParameterValue` Mat "DepthRT" (`SceneCaptureComponent2D.TextureTarget` (`self.SceneCaptureComponent2D`)))
  (`MaterialInstanceDynamic.SetScalarParameterValue` Mat "ResY/X" (`self.RexY/X`))
  (`MaterialInstanceDynamic.SetScalarParameterValue` Mat "FOV" (`self.Field Of View`))
  (`MaterialInstanceDynamic.SetScalarParameterValue` Mat "MaxDistacne" (`self.MaxDistacne`))
  (`MaterialInstanceDynamic.SetVectorParameterValue` Mat "Camera Relative Position (V3)" (`KismetMathLibrary.Conv_VectorToLinearColor` (`SceneComponent.K2_GetComponentLocation` _scenecapturecomponent2d)))
  (`MaterialInstanceDynamic.SetVectorParameterValue` Mat "X Camera to World Vector (V3)" (`KismetMathLibrary.Conv_VectorToLinearColor` (`SceneComponent.GetRightVector` _scenecapturecomponent2d)))
  (`MaterialInstanceDynamic.SetVectorParameterValue` Mat "Y Camera to World Vector (V3)" (`KismetMathLibrary.Conv_VectorToLinearColor` (* (`SceneComponent.GetUpVector` _scenecapturecomponent2d) -1.0)))
  (`MaterialInstanceDynamic.SetVectorParameterValue` Mat "Z Camera to World Vector (V3)" (`KismetMathLibrary.Conv_VectorToLinearColor` (`SceneComponent.GetForwardVector` _scenecapturecomponent2d))))

(fn `UserConstructionScript`
  (bind _maxdistacne (`self.MaxDistacne`))
  (bind _scenecapturecomponent2d (`self.SceneCaptureComponent2D`))
  (bind _reslution (`self.Reslution`))
  (bind _decal (`self.Decal`))
  (bind _returnvalue (* _maxdistacne 0.5))
  (`SceneComponent.SetWorldScale3D` _decal (`KismetMathLibrary.MakeVector` (* _maxdistacne (`self.RexY/X`)) _maxdistacne _returnvalue))
  (`SceneComponent.K2_SetRelativeLocation` _decal (`KismetMathLibrary.MakeVector` _returnvalue) false false)
  (`SceneComponent.SetWorldScale3D` (`self.Sphere`) (`KismetMathLibrary.Conv_DoubleToVector` (/ (`self.MaxDistacne`) 50.0)))
  (bind _returnvalue_2 (`KismetRenderingLibrary.CreateRenderTarget2D` _reslution (`KismetMathLibrary.FTrunc` (* _reslution (`self.RexY/X`))) "RTF_R16f"))
  (set `SceneCaptureComponent2D.TextureTarget` _returnvalue_2 _scenecapturecomponent2d)
  (set `SceneCaptureComponent2D.FOVAngle` (`self.Field Of View`) _scenecapturecomponent2d)
  (set `SceneCaptureComponent.MaxViewDistanceOverride` (`self.MaxDistacne`) _scenecapturecomponent2d)
  (bind _returnvalue_3 (`DecalComponent.CreateDynamicMaterialInstance` (`self.Decal`)))
  (`self.SetCameraParameters` _returnvalue_3)
  (bind _returnvalue_4 (`PrimitiveComponent.CreateDynamicMaterialInstance` (`self.Sphere`) 0 "/Game/LF_VisualField/M_DeBug.M_DeBug" "None"))
  (`self.SetCameraParameters` _returnvalue_4))