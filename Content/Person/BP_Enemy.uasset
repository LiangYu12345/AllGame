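; BP_Enemy is an enemy actor that reports its position relative to the player controller to the HUD for an icon.
; Shortly after BeginPlay it attaches its CalHelper component to the player controller's root, using that component to convert world position into controller-local space.
; Every tick it moves CalHelper to the enemy's location and sends the resulting relative X and Y to the HUD through UpdateIconPositionMessage.
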(event `self.ReceiveBeginPlay`
  (`KismetSystemLibrary.Delay` 0.2)
  (`SceneComponent.K2_AttachToComponent` (`self.cal_helper`) (`Actor.RootComponent` (`GameplayStatics.GetPlayerController` 0)) "None" "KeepRelative" "KeepRelative" "KeepRelative" true)
  (`self.Update Icon Positon`))

(event `self.ReceiveTick`
  (params (DeltaSeconds :type "Float (single-precision)"))
  (`self.Update Icon Positon`))

(fn `Update Icon Positon`
  (`SceneComponent.K2_SetWorldLocation` (`self.cal_helper`) (`self.K2_GetActorLocation`) false false)
  (message `/Game/Person/miniMap_Interface.UpdateIconPosition` (`PlayerController.GetHUD` (`GameplayStatics.GetPlayerController` 0)) (`KismetMathLibrary.Conv_VectorToVector2D` (`SceneComponent.RelativeLocation` (`self.cal_helper`)))))

(fn `UserConstructionScript`)