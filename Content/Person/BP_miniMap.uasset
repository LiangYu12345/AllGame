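; Map manager that puts the HUD_Person widget on screen and runs the player's minimap and toggleable full map.
; Tick writes player location and normalized yaw into the M_miniMap material parameter collection.
; ToggleMap shows or removes HUD_FullMap, creating an icon widget for each MapItem_Interface actor.
; While the map shows, Tick re-queries those actors and pairs them with icons by array index to update position and angle.
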(event `self.ReceiveBeginPlay`
  (bind _returnvalue (`|CreateWidget` "/Game/Person/HUD_Person.HUD_Person_C"))
  (`/Engine/EditorBlueprintResources/StandardMacros.IsValid` _returnvalue
    (:`Is Valid`
      (`UserWidget.AddToViewport` _returnvalue 0)
      (set `self.miniMap` _returnvalue))))

(event `self.ReceiveTick`
  (params (DeltaSeconds :type "Float (single-precision)"))
  (bind _returnvalue (`GameplayStatics.GetPlayerCharacter` 0))
  (bind (_returnvalue_roll _returnvalue_pitch _returnvalue_yaw) (`KismetMathLibrary.BreakRotator` (`self.K2_GetActorRotation` _returnvalue)))
  (`|ExecutionSequence`
    (:`then_0`
      (`KismetMaterialLibrary.SetVectorParameterValue` "/Game/Person/Asset/Material/M_miniMap.M_miniMap" "Location" (`KismetMathLibrary.Conv_VectorToLinearColor` (`self.K2_GetActorLocation` _returnvalue)))
      (`KismetMaterialLibrary.SetScalarParameterValue` "/Game/Person/Asset/Material/M_miniMap.M_miniMap" "Yaw" (/ (`KismetMathLibrary.SelectFloat` (+ _returnvalue_yaw 360.0) _returnvalue_yaw (< _returnvalue_yaw 0.0)) 360.0)))
    (:`then_1`
      (if (`self.fullMapShow`)
        (bind _outactors (`GameplayStatics.GetAllActorsWithInterface` "/Game/Person/MapItem_Interface.MapItem_Interface_C"))
        (for (_array_element _array_index) _outactors
          (for (_array_element_2 _array_index_2) (`self.mapIcons`)
            (if (== _array_index_2 _array_index)
              (break)))
          (bind _asfull_map_icon (cast `/Game/Person/fullMap_Icon` _array_element_2))
          (bind (_location _icon _icon_size _yaw) (message `/Game/Person/MapItem_Interface.GetMapItemData` _array_element))
          (`/Game/Person/fullMap_Icon.Update FullMap Icon` _asfull_map_icon (`KismetMathLibrary.Conv_VectorToVector2D` _location) _yaw))))))

(event `/Game/Person/fullMap_Interface.ToggleMap`
  (params (enable :type Boolean))
  (bind _mapicons (`self.mapIcons`))
  (if enable
    (`self.fullMap`
      (:`then`
        _)
      (:`else`
        (bind _returnvalue (`|CreateWidget` "/Game/Person/HUD_FullMap.HUD_FullMap_C"))
        (bind _output_get (set `self.fullMap` _returnvalue))))
    (`UserWidget.AddToViewport` _output_get 0)
    (set `self.fullMapShow` true)
    (bind _outactors (`GameplayStatics.GetAllActorsWithInterface` "/Game/Person/MapItem_Interface.MapItem_Interface_C"))
    (for _array_element _outactors
      (bind _returnvalue_2 (`|CreateWidget` "/Game/Person/fullMap_Icon.fullMap_Icon_C"))
      (bind (_location _icon _icon_size _yaw) (message `/Game/Person/MapItem_Interface.GetMapItemData` _array_element))
      (`/Game/Person/fullMap_Icon.Init FullMap Icon` _returnvalue_2 _icon (`KismetMathLibrary.Conv_VectorToVector2D` _location) _icon_size _yaw)
      (`UserWidget.AddToViewport` _returnvalue_2 0)
      (`KismetArrayLibrary.Array_Add` (`self.mapIcons`) _returnvalue_2))
    (else
      (bind _fullmap (`self.fullMap`)
        (:`then`
          (if (`Widget.IsInViewport` _fullmap)
            (`Widget.RemoveFromParent` _fullmap)
            (for _array_element_2 _mapicons
              (`Widget.RemoveFromParent` _array_element_2)
              (set `self.fullMapShow` false))
            (`KismetArrayLibrary.Array_Clear` _mapicons)))
        (:`else`)))))

(fn `UserConstructionScript`)