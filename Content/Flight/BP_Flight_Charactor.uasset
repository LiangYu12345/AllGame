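; Flyable plane character with a ground-roll mode and a flight mode, switched on IsFlying.
; Forward input moves it flat along the ground, or adjusts a clamped target speed in flight, which Tick eases toward and applies along the mesh's forward vector.
; The take-off branch enables spring-arm lag and lifts the plane, but sets IsFlying false and checks an unset key.
; BeginPlay deactivates wing and jet Niagara effects; right input is empty.
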(event `self.ReceiveTick`
  (params (DeltaSeconds :type "Float (single-precision)"))
  ;[1 1 1] for ground movement. Interp value to low value as flight should speed up very gradually when on ground
  (`|ExecutionSequence`
    (:`then_0`
      (bind _output_get (set `self.Move Forward Interp` (`KismetMathLibrary.ClampAngle` (`KismetMathLibrary.FInterpTo` (stale _output_get) (`self.Move Forward Interp`) (`GameplayStatics.GetWorldDeltaSeconds`) 0.2) 0.0 1.0))))
    (:`then_1`
      (if (`self.isFlying`)
        (`self.Add flight movement`)))))

(event `self.ReceiveBeginPlay`
  ;[1 1 1] init min fly speed to 2500
  (`|ExecutionSequence`
    (:`then_0`
      (set `self.MinFlySpeed` (`self.MinFlySpeed`))
      ;[1 1 1] init hide all Niagara
      (`ActorComponent.SetActive` (`self.Wing_Left`) false false)
      (`ActorComponent.SetActive` (`self.Wing_Right`) false false)
      (`ActorComponent.SetActive` (`self.NS_West_Fighter_Typhoon_JetLeft`) false false)
      (`ActorComponent.SetActive` (`self.NS_West_Fighter_Typhoon_JetRight`) false false))
    (:`then_1`
      (`SceneComponent.SetRelativeScale3D` (`self.NS_West_Fighter_Typhoon_JetLeft`) (0.0 0.0 0.0))
      (`SceneComponent.SetRelativeScale3D` (`self.NS_West_Fighter_Typhoon_JetRight`) (0.0 0.0 0.0)))))

(event `InputAxis|MoveForward` :overrideparent false
  (params (AxisValue :type "Float (single-precision)"))
  (bind _springarm (`self.SpringArm`))
  ;[1 1 1] if  flying , then move forward inputs should increase/decrease flight speed. if not then it will add movement on floor using offset
  (if (`self.isFlying`)
    (set `self.TargetFlySpeed` (`KismetMathLibrary.FClamp` (+ (* AxisValue (`GameplayStatics.GetWorldDeltaSeconds`) 1500.0) (`self.TargetFlySpeed`)) (`self.MinFlySpeed`) (`self.MaxFlySpeed`))))
  (if (not (`self.isFlying`))
    (`|ExecutionSequence`
      (:`then_0`
        ;[1 1 1] Slowly move plane across ground , with speed getting higher the longer move forward is held down. Z is zero-ed out since it should not move up and only on same ground
        (`self.K2_AddActorWorldOffset` (`KismetMathLibrary.MakeVector` (.x (* (`self.GetActorForwardVector`) (`self.Move Forward Interp`) (/ (`self.TargetFlySpeed`) 500.0))) (.y (* (`self.GetActorForwardVector`) (`self.Move Forward Interp`) (/ (`self.TargetFlySpeed`) 500.0)))) true)
        ;[1 1 1] if moveing fast enough on ground and space is pressed, then plane will go into flying mode.lag is turned on for spring arm for smotther amera flight controls and small offset added to prevent crashing on ground immediately upon take-off
        (if (and (> (`self.Move Forward Interp`) 0.7) (`PlayerController.IsInputKeyDown` (`GameplayStatics.GetPlayerController` 0) "None"))
          (set `self.isFlying` false)
          (bind _output_get (set `SpringArmComponent.bEnableCameraLag` true _springarm))
          (set `SpringArmComponent.bEnableCameraRotationLag` _output_get _springarm)
          (set `SpringArmComponent.bUsePawnControlRotation` false _springarm)
          (`self.K2_AddActorWorldOffset` (0.0 0.0 25.0) true))))))

(event `InputAxis|MoveRight` :overrideparent false
  (params (AxisValue :type "Float (single-precision)")))

(fn `Add flight movement`
  (bind _returnvalue (`GameplayStatics.GetWorldDeltaSeconds`))
  ;[1 1 1] interp set Flight speed
  (bind _output_get (set `self.CurrentFlySpeed` (`KismetMathLibrary.FInterpTo` (stale _output_get) (`self.TargetFlySpeed`) _returnvalue 8.0)))
  ;[1 1 1] Add movement in forward direciton to plane
  (`self.K2_AddActorWorldOffset` (* (`SceneComponent.GetForwardVector` (`self.Mesh`)) (* _output_get _returnvalue))))

(fn `UserConstructionScript`)